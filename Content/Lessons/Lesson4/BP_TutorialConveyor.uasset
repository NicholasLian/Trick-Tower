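; BP_TutorialConveyor is a lesson conveyor that pushes whatever sits inside its Box trigger along its Arrow's forward direction.
; Box overlap events maintain lists of overlapping actors and components.
; Each Tick offsets every actor by a fixed step, unswept and unscaled by delta time.
; Nested inside that loop, static mesh components receive an acceleration-style force, so it repeats once per listed actor.
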(event `self.Box.OnComponentBeginOverlap`
  (params (OverlappedComponent :type "PrimitiveComponent Object Reference") (OtherActor :type "Actor Object Reference") (OtherComp :type "PrimitiveComponent Object Reference") (OtherBodyIndex :type Integer) (bFromSweep :type Boolean) (SweepResult :type "HitResult Structure (by ref)"))
  (`KismetArrayLibrary.Array_Add` (`self.Components`) OtherComp)
  (`KismetArrayLibrary.Array_Add` (`self.Actors`) OtherActor))

(event `self.Box.OnComponentEndOverlap`
  (params (OverlappedComponent :type "PrimitiveComponent Object Reference") (OtherActor :type "Actor Object Reference") (OtherComp :type "PrimitiveComponent Object Reference") (OtherBodyIndex :type Integer))
  (`KismetArrayLibrary.Array_RemoveItem` (`self.Components`) OtherComp)
  (`KismetArrayLibrary.Array_RemoveItem` (`self.Actors`) OtherActor))

(event `self.ReceiveTick`
  (params (DeltaSeconds :type "Float (single-precision)"))
  (for _array_element (`self.Actors`)
    (`self.K2_SetActorLocation` _array_element (+ (`self.K2_GetActorLocation` _array_element) (* (`SceneComponent.GetForwardVector` (`self.Arrow`)) 10.0)) false false)
    (for _array_element_2 (`self.Components`)
      (bind _asstatic_mesh_component (cast `StaticMeshComponent` _array_element_2))
      (`PrimitiveComponent.AddForce` _asstatic_mesh_component (* (`SceneComponent.GetForwardVector` (`self.Arrow`)) 200.0) "None" true))))

(fn `UserConstructionScript`)