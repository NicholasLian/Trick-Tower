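; BP_PointAndClick is a lesson character for point-and-click teleport locomotion with snap turning, apparently for a VR player.
; Each tick, unless right mouse is held, scaled mouse delta drives BPCMouseCursor, coloured green or red by whether CharacterMovement deems the hit walkable.
; The Teleport action moves the actor to a valid cursor location, raised by the capsule half-height.
; Holding right mouse accumulates Turn input and calls TurnVRPlayer in fixed steps past a threshold.
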(event `self.ReceiveTick`
  (params (DeltaSeconds :type "Float (single-precision)"))
  (bind (_deltax _deltay) (`PlayerController.GetInputMouseDelta` (`GameplayStatics.GetPlayerController` 0)))
  (if (not (`self.Can Turn`))
    (bind _tracehit (`/Game/Blueprints/Utility/BPC_MouseCursor.Update` (`self.BPC_MouseCursor`) (/ _deltax 3.0) (/ _deltay 3.0)))
    (bind _output_get (set `self.Can Teleport` (`CharacterMovementComponent.IsWalkable` (`self.CharacterMovement`) _tracehit)))
    (if _output_get
      (`/Game/Blueprints/Utility/BPC_MouseCursor.SetCursorColor` (`self.BPC_MouseCursor`) (struct :`G` 0.78 :`B` 0.052098 :`A` 1.0))
      (else
        (`/Game/Blueprints/Utility/BPC_MouseCursor.SetCursorColor` (`self.BPC_MouseCursor`) (struct :`R` 0.815 :`G` 0.020375 :`B` 0.020375 :`A` 1.0))))))

(event `InputAction|Teleport`
  (params (Key :type "Key Structure" :default "AnyKey"))
  (:`Pressed`
    (if (`self.Can Teleport`)
      (`self.K2_SetActorLocation` (+ (`/Game/Blueprints/Utility/BPC_MouseCursor.GetCursorLocation` (`self.BPC_MouseCursor`)) (`KismetMathLibrary.MakeVector` 0.0 0.0 (`CapsuleComponent.GetScaledCapsuleHalfHeight` (`self.CapsuleComponent`))))))))

(event `Key|RightMouseButton`
  (params (Key :type "Key Structure" :default "AnyKey"))
  (:`Pressed`
    (set `self.Can Turn` true))
  (:`Released`
    (set `self.Can Turn` false)))

(event `InputAxis|Turn`
  (params (AxisValue :type "Float (single-precision)"))
  (if (`self.Can Turn`)
    (bind _output_get (set `self.Turn Mouse Delta` (+ AxisValue (`self.Turn Mouse Delta`))))
    (if (> _output_get 5.0)
      (`/Game/Blueprints/Utility/LayoutVRUtilityFunctions.Turn VR Player` 20.0)
      (set `self.Turn Mouse Delta` 0.0 :!label _label)
      (elif (< _output_get -5.0)
        (`/Game/Blueprints/Utility/LayoutVRUtilityFunctions.Turn VR Player` -20.0)
        (goto _label)))))

(fn `UserConstructionScript`)