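; BP_25DCamera1 is a side-scrolling 2.5D camera actor that follows the first player character in a lesson level.
; On BeginPlay it records its starting offset from the character.
; Every Tick it moves to the character's X and Z plus that offset, with Y built from a hard-coded value plus the offset, so depth stays constant.
; The X and Y locations saved at BeginPlay do not feed the movement.
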(event `self.ReceiveBeginPlay`
  (bind _returnvalue (`self.K2_GetActorLocation`))
  (set `self.Camera Offset` (- _returnvalue (`self.K2_GetActorLocation` (`GameplayStatics.GetPlayerCharacter` 0))))
  (set `self.Camera X Location` (.x _returnvalue))
  (set `self.Camera Y Location` (.y _returnvalue)))

(event `self.ReceiveTick`
  (params (DeltaSeconds :type "Float (single-precision)"))
  (bind _returnvalue (`GameplayStatics.GetPlayerCharacter` 0))
  (bind (_returnvalue_x _returnvalue_y _returnvalue_z) (`KismetMathLibrary.BreakVector` (`self.K2_GetActorLocation` _returnvalue)))
  (`/Engine/EditorBlueprintResources/StandardMacros.IsValid` _returnvalue
    (:`Is Valid`
      (`self.K2_SetActorLocation` (+ (`KismetMathLibrary.MakeVector` _returnvalue_x -500.0 _returnvalue_z) (`self.Camera Offset`))))))

(fn `UserConstructionScript`)