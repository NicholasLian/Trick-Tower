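; BP_25DCamera_Down is a camera actor, apparently for a 2.5D pipe game lesson, that follows player character 0.
; BeginPlay records its starting offset from the character, and Tick moves it to the character's current location plus that offset on all three axes, without smoothing.
; It also caches its starting X in CameraXLocation, but nothing in these graphs reads that value.
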(event `self.ReceiveBeginPlay`
  (bind _returnvalue (`self.K2_GetActorLocation`))
  (set `self.Camera Offset` (- _returnvalue (`self.K2_GetActorLocation` (`GameplayStatics.GetPlayerCharacter` 0))))
  (set `self.Camera X Location` (.x _returnvalue)))

(event `self.ReceiveTick`
  (params (DeltaSeconds :type "Float (single-precision)"))
  (`self.K2_SetActorLocation` (+ (`KismetMathLibrary.MakeVector` (.x (`self.K2_GetActorLocation` (`GameplayStatics.GetPlayerCharacter` 0))) (.y (`self.K2_GetActorLocation` (`GameplayStatics.GetPlayerCharacter` 0))) (.z (`self.K2_GetActorLocation` (`GameplayStatics.GetPlayerCharacter` 0)))) (`self.Camera Offset`))))

(fn `UserConstructionScript`)