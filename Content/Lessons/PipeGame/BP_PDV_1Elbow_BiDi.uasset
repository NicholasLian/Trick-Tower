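; Bidirectional 90-degree elbow tube for a pipe game that pushes physics mesh components through it and can rotate a quarter turn.
; Four trigger spheres track overlapping components; each Tick pushes the most recently entered sphere's list along its matching arrow.
; The first end entered, A1 or A4, sets forward or reversed force and a glass material until the opposite end clears it.
; RotateVentInterface starts the one-second timed turn, refusing while busy.
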(event `self.ReceiveBeginPlay`
  (set `self.SphereIndex` 0)
  (set `self.1stEntryIndex` 0)
  (set `self.ArrowArray` (`|MakeArray` (`self.ArrowA1`) (`self.ArrowA2`) (`self.ArrowA3`) (`self.ArrowA4`)))
  (set `self.EntryKey` "N0"))

(event `self.ReceiveTick`
  (params (DeltaSeconds :type "Float (single-precision)"))
  (`self.RotateVent`)
  (`self.GetComponentArray`)
  (`self.GetCurrentArrow`)
  (for _array_element (`self.CurrentComponentList`)
    (set `self.CurrentObject` _array_element)
    (`self.AddForceToComponents`)))

(event `self.SphereCollisionA1.OnComponentBeginOverlap`
  (params (OverlappedComponent :type "PrimitiveComponent Object Reference") (OtherActor :type "Actor Object Reference") (OtherComp :type "PrimitiveComponent Object Reference") (OtherBodyIndex :type Integer) (bFromSweep :type Boolean) (SweepResult :type "HitResult Structure (by ref)"))
  (bind _returnvalue (`KismetStringLibrary.EqualEqual_StrStr` (`self.EntryKey`) (`KismetMathLibrary.SelectString` "N0" "" true)))
  ;[1 1 1] Overlap Triggers
  (`KismetArrayLibrary.Array_Add` (`self.ComponentsA1`) OtherComp)
  (set `self.SphereIndex` 1)
  (if _returnvalue
    (set `self.EntryKey` "A1")
    (`PrimitiveComponent.SetMaterial` (`self.Tube90SE`) 0 "/Game/Materials/Architecture/Glass/MI_Glass_Hex_B.MI_Glass_Hex_B")
    (if _returnvalue :!label _label
      (set `self.EntryKey` "A4")
      (`PrimitiveComponent.SetMaterial` (`self.Tube90SE`) 0 "/Game/Materials/Architecture/Glass/MI_Glass_Hex_B.MI_Glass_Hex_B"))))

(event `self.SphereCollisionA2.OnComponentBeginOverlap`
  (params (OverlappedComponent :type "PrimitiveComponent Object Reference") (OtherActor :type "Actor Object Reference") (OtherComp :type "PrimitiveComponent Object Reference") (OtherBodyIndex :type Integer) (bFromSweep :type Boolean) (SweepResult :type "HitResult Structure (by ref)"))
  ;[1 1 1] Overlap Triggers
  (`KismetArrayLibrary.Array_Add` (`self.ComponentsA2`) OtherComp)
  (set `self.SphereIndex` 2))

(event `self.SphereCollisionA3.OnComponentBeginOverlap`
  (params (OverlappedComponent :type "PrimitiveComponent Object Reference") (OtherActor :type "Actor Object Reference") (OtherComp :type "PrimitiveComponent Object Reference") (OtherBodyIndex :type Integer) (bFromSweep :type Boolean) (SweepResult :type "HitResult Structure (by ref)"))
  ;[1 1 1] Overlap Triggers
  (`KismetArrayLibrary.Array_Add` (`self.ComponentsA3`) null)
  (set `self.SphereIndex` 3))

(event `self.SphereCollisionA4.OnComponentBeginOverlap`
  (params (OverlappedComponent :type "PrimitiveComponent Object Reference") (OtherActor :type "Actor Object Reference") (OtherComp :type "PrimitiveComponent Object Reference") (OtherBodyIndex :type Integer) (bFromSweep :type Boolean) (SweepResult :type "HitResult Structure (by ref)"))
  ;[1 1 1] Overlap Triggers
  (`KismetArrayLibrary.Array_Add` (`self.ComponentsA4`) OtherComp)
  (set `self.SphereIndex` 4)
  (goto _label))

(event `self.SphereCollisionA1.OnComponentEndOverlap`
  (params (OverlappedComponent :type "PrimitiveComponent Object Reference") (OtherActor :type "Actor Object Reference") (OtherComp :type "PrimitiveComponent Object Reference") (OtherBodyIndex :type Integer))
  ;[1 1 1] Overlap Triggers
  (`KismetArrayLibrary.Array_RemoveItem` (`self.ComponentsA1`) OtherComp)
  (if (`KismetStringLibrary.EqualEqual_StrStr` (`self.EntryKey`) "A4")
    (set `self.EntryKey` (`KismetMathLibrary.SelectString` "N0" "" true))
    (`PrimitiveComponent.SetMaterial` (`self.Tube90SE`) 0 "/Engine/EditorMeshes/ColorCalibrator/M_ClearCoat.M_ClearCoat")))

(event `self.SphereCollisionA2.OnComponentEndOverlap`
  (params (OverlappedComponent :type "PrimitiveComponent Object Reference") (OtherActor :type "Actor Object Reference") (OtherComp :type "PrimitiveComponent Object Reference") (OtherBodyIndex :type Integer))
  ;[1 1 1] Overlap Triggers
  (`KismetArrayLibrary.Array_RemoveItem` (`self.ComponentsA2`) OtherComp))

(event `self.SphereCollisionA3.OnComponentEndOverlap`
  (params (OverlappedComponent :type "PrimitiveComponent Object Reference") (OtherActor :type "Actor Object Reference") (OtherComp :type "PrimitiveComponent Object Reference") (OtherBodyIndex :type Integer))
  ;[1 1 1] Overlap Triggers
  (`KismetArrayLibrary.Array_RemoveItem` (`self.ComponentsA3`) null))

(event `self.SphereCollisionA4.OnComponentEndOverlap`
  (params (OverlappedComponent :type "PrimitiveComponent Object Reference") (OtherActor :type "Actor Object Reference") (OtherComp :type "PrimitiveComponent Object Reference") (OtherBodyIndex :type Integer))
  ;[1 1 1] Overlap Triggers
  (`KismetArrayLibrary.Array_RemoveItem` (`self.ComponentsA4`) OtherComp)
  (if (`KismetStringLibrary.EqualEqual_StrStr` (`self.EntryKey`) "A1")
    (set `self.EntryKey` (`KismetMathLibrary.SelectString` "N0" "" true))
    (`PrimitiveComponent.SetMaterial` (`self.Tube90SE`) 0 "/Engine/EditorMeshes/ColorCalibrator/M_ClearCoat.M_ClearCoat")))

(event `RotateVent`
  ;[1 1 1] Rotate Self
  (if (`self.CanRotate`)
    (bind _output_get (set `self.Difference` (- (`KismetSystemLibrary.GetGameTimeInSeconds`) (`self.TriggerTime`))))
    (if (not (<= _output_get 1.0))
      (set `self.CanRotate` false)
      (set `self.Difference` 1.0))
    (`SceneComponent.K2_SetWorldRotation` (`self.CircularBase`) (`KismetMathLibrary.ComposeRotators` (`KismetMathLibrary.MakeRotator` 0.0 0.0 (* (`self.Difference`) 90.0)) (`self.WorldRotation`)) false false)))

(event `AddForceToComponents`
  (bind _returnvalue (`KismetMathLibrary.SelectFloat` 6400.0 0.0 true))
  (bind _entrykey (`self.EntryKey`))
  (bind _returnvalue_2 (`SceneComponent.GetForwardVector` (`self.CurrentArrow`)))
  (bind _asstatic_mesh_component (cast `StaticMeshComponent` (`self.CurrentObject`)))
  (switch `string` _entrykey
    (:`Default`
      (`KismetSystemLibrary.PrintString` "EntryKeyError!" true true (struct :`G` 1.0 :`A` 1.0) 5.0)
      (`KismetSystemLibrary.PrintString` _entrykey true true (struct :`G` 1.0 :`A` 1.0) 5.0))
    (:`A1`
      (`PrimitiveComponent.AddForce` _asstatic_mesh_component (* _returnvalue_2 _returnvalue) "None" false))
    (:`A4`
      (`PrimitiveComponent.AddForce` _asstatic_mesh_component (* (* _returnvalue_2 -1) _returnvalue) "None" false))))

(event `GetComponentArray`
  (switch `int` (`self.SphereIndex`)
    (:`1`
      (set `self.CurrentComponentList` (`self.ComponentsA1`)))
    (:`2`
      (set `self.CurrentComponentList` (`self.ComponentsA2`)))
    (:`3`
      (set `self.CurrentComponentList` (`self.ComponentsA3`)))
    (:`4`
      (set `self.CurrentComponentList` (`self.ComponentsA4`)))))

(event `GetCurrentArrow`
  (set `self.CurrentArrow` (`KismetArrayLibrary.Array_Get` (`self.ArrowArray`) (- (`self.SphereIndex`) 1))))

(fn `RotateVentInterface`
  (returns (Boolean :type Boolean))
  (if (`self.CanRotate`)
    (`KismetSystemLibrary.PrintString` "BUSY!!!" true true (struct :`G` 0.5 :`A` 1.0) 2.0)
    (return false)
    (else
      (set `self.CanRotate` true)
      (set `self.TriggerTime` (`KismetSystemLibrary.GetGameTimeInSeconds`))
      (set `self.WorldRotation` (`SceneComponent.K2_GetComponentRotation` (`self.CircularBase`))) ; Set upon trigger
      (return false))))

(fn `UserConstructionScript`)