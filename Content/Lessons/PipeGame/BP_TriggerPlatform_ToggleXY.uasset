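; Trigger platform in the PipeGame lesson that changes the X or Y value of a referenced BP_MemoryCube when its box is overlapped.
; IsX selects ToggleX or ToggleY, and IsIncrease sets the boolean passed to that call.
; Overlap begin turns both meshes green and plays a laser sound; overlap end turns them blue and plays a chime.
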(event `self.Box.OnComponentBeginOverlap`
  (params (OverlappedComponent :type "PrimitiveComponent Object Reference") (OtherActor :type "Actor Object Reference") (OtherComp :type "PrimitiveComponent Object Reference") (OtherBodyIndex :type Integer) (bFromSweep :type Boolean) (SweepResult :type "HitResult Structure (by ref)"))
  (bind _isincrease (`self.IsIncrease`))
  (bind _memorycube (`self.MemoryCube`))
  (`MeshComponent.SetVectorParameterValueOnMaterials` (`self.StaticMesh1`) "Color" (`KismetMathLibrary.Conv_LinearColorToVector` (struct :`G` 1.0 :`A` 1.0)))
  (`MeshComponent.SetVectorParameterValueOnMaterials` (`self.StaticMesh2`) "Color" (`KismetMathLibrary.Conv_LinearColorToVector` (struct :`G` 1.0 :`A` 1.0)))
  (`AudioComponent.Play` (`self.SW_Laser_3`) 0.0)
  (if (`self.IsX`)
    (if _isincrease
      (bind _asbp_memory_cube (cast `/Game/Lessons/PipeGame/BP_MemoryCube` _memorycube))
      (`/Game/Lessons/PipeGame/BP_MemoryCube.ToggleX` _asbp_memory_cube true)
      (else
        (bind _asbp_memory_cube_2 (cast `/Game/Lessons/PipeGame/BP_MemoryCube` _memorycube))
        (`/Game/Lessons/PipeGame/BP_MemoryCube.ToggleX` _asbp_memory_cube_2 false)))
    (elif _isincrease
      (bind _asbp_memory_cube_3 (cast `/Game/Lessons/PipeGame/BP_MemoryCube` _memorycube))
      (`/Game/Lessons/PipeGame/BP_MemoryCube.ToggleY` _asbp_memory_cube_3 true)
      (else
        (bind _asbp_memory_cube_4 (cast `/Game/Lessons/PipeGame/BP_MemoryCube` _memorycube))
        (`/Game/Lessons/PipeGame/BP_MemoryCube.ToggleY` _asbp_memory_cube_4 false)))))

(event `self.Box.OnComponentEndOverlap`
  (params (OverlappedComponent :type "PrimitiveComponent Object Reference") (OtherActor :type "Actor Object Reference") (OtherComp :type "PrimitiveComponent Object Reference") (OtherBodyIndex :type Integer))
  (`MeshComponent.SetVectorParameterValueOnMaterials` (`self.StaticMesh1`) "Color" (`KismetMathLibrary.Conv_LinearColorToVector` (struct :`G` 0.287324 :`B` 1.0 :`A` 1.0)))
  (`MeshComponent.SetVectorParameterValueOnMaterials` (`self.StaticMesh2`) "Color" (`KismetMathLibrary.Conv_LinearColorToVector` (struct :`G` 0.287324 :`B` 1.0 :`A` 1.0)))
  (`AudioComponent.Play` (`self.SW_Chime_1`) 0.0))

(fn `UserConstructionScript`)