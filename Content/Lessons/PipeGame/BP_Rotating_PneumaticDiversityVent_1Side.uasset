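; Rotating one-sided pneumatic vent for the pipe game that blows overlapping objects along its arrow.
; Components overlapping the collision box are tracked in an array, and static meshes among them receive a constant force every Tick.
; RotateVent records the start time and rotation, then Tick turns the box a quarter turn in pitch over one second, refusing new triggers meanwhile.
; Overlap also swaps the PlaneF material, with no revert.
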(event `self.ReceiveTick`
  (params (DeltaSeconds :type "Float (single-precision)"))
  (if (`self.CanRotate`)
    ;[1 1 1] Rotate Self
    (bind _output_get (set `self.Difference` (- (`KismetSystemLibrary.GetGameTimeInSeconds`) (`self.TriggerTime`))))
    (if (not (<= _output_get 1.0))
      (set `self.CanRotate` false)
      (set `self.Difference` 1.0))
    (`SceneComponent.K2_SetWorldRotation` (`self.CollisionBox`) (`KismetMathLibrary.ComposeRotators` (`KismetMathLibrary.MakeRotator` 0.0 (* (`self.Difference`) 90.0)) (`self.WorldRotation`)) false false))
  ;[1 1 1] Add Force to Components
  (for _array_element (`self.Components`)
    (bind _asstatic_mesh_component (cast `StaticMeshComponent` _array_element))
    (`PrimitiveComponent.AddForce` _asstatic_mesh_component (* (`SceneComponent.GetForwardVector` (`self.Arrow`)) 160000.0) "None" false)))

(event `self.CollisionBox.OnComponentBeginOverlap`
  (params (OverlappedComponent :type "PrimitiveComponent Object Reference") (OtherActor :type "Actor Object Reference") (OtherComp :type "PrimitiveComponent Object Reference") (OtherBodyIndex :type Integer) (bFromSweep :type Boolean) (SweepResult :type "HitResult Structure (by ref)"))
  (`KismetArrayLibrary.Array_Add` (`self.Components`) OtherComp)
  ;[1 1 1] Set Material
  (`KismetSystemLibrary.PrintString` "SetMaterial")
  (`PrimitiveComponent.SetMaterial` (`self.Plane_F`) 0 "/Game/Materials/Architecture/Metal/Bare/MI_Metal_Brushed_001_a.MI_Metal_Brushed_001_a"))

(event `self.CollisionBox.OnComponentEndOverlap`
  (params (OverlappedComponent :type "PrimitiveComponent Object Reference") (OtherActor :type "Actor Object Reference") (OtherComp :type "PrimitiveComponent Object Reference") (OtherBodyIndex :type Integer))
  (bind _components (`self.Components`))
  (`KismetArrayLibrary.Array_RemoveItem` _components OtherComp)
  ;[1 1 1] Set Material
  (if (<= (`KismetArrayLibrary.Array_Length` _components) 0)
    _))

(event `RotateVent`
  (if (`self.CanRotate`)
    (`KismetSystemLibrary.PrintString` "Sorry!" true true (struct :`G` 0.5 :`A` 1.0))
    (else
      (set `self.CanRotate` true)
      (set `self.TriggerTime` (`KismetSystemLibrary.GetGameTimeInSeconds`))
      (`KismetSystemLibrary.PrintString` "Rotating")
      (set `self.WorldRotation` (`SceneComponent.K2_GetComponentRotation` (`self.CollisionBox`))) ; Set upon trigger
    )))

(fn `UserConstructionScript`)