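; Curved pipe launcher for the pipe game that pushes static mesh objects along the arrow directions inside its Tube90.
; Four sphere triggers each track their overlapping components and register their index while occupied.
; Every Tick, each occupied sphere applies a constant force along its child arrow, found through Tube90's component hierarchy by index.
; Entering the first sphere swaps the tube to hex glass; emptying the last sets clear coat.
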(event `self.ReceiveBeginPlay`
  (set `self.Index` 0))

(event `self.ReceiveTick`
  (params (DeltaSeconds :type "Float (single-precision)"))
  (for _array_element (`self.CollisionIndexes`)
    (set `self.Index` _array_element) ; Represents Current Sphere Collision
    (`self.GetComponentArray`)
    (`self.GetCurrentArrow`)
    (for _array_element_2 (`self.CurrentComponentList`)
      (set `self.CurrentObject` _array_element_2)
      (`self.AddForceToComponents`))))

(event `self.SphereCollision1.OnComponentBeginOverlap`
  (params (OverlappedComponent :type "PrimitiveComponent Object Reference") (OtherActor :type "Actor Object Reference") (OtherComp :type "PrimitiveComponent Object Reference") (OtherBodyIndex :type Integer) (bFromSweep :type Boolean) (SweepResult :type "HitResult Structure (by ref)"))
  ;[1 1 1] Overlap Triggers
  (`KismetArrayLibrary.Array_Add` (`self.Components1`) OtherComp)
  (`KismetArrayLibrary.Array_AddUnique` (`self.CollisionIndexes`) 1)
  (`PrimitiveComponent.SetMaterial` (`self.Tube90`) 0 "/Game/Materials/Architecture/Glass/MI_Glass_Hex_B.MI_Glass_Hex_B"))

(event `self.SphereCollision2.OnComponentBeginOverlap`
  (params (OverlappedComponent :type "PrimitiveComponent Object Reference") (OtherActor :type "Actor Object Reference") (OtherComp :type "PrimitiveComponent Object Reference") (OtherBodyIndex :type Integer) (bFromSweep :type Boolean) (SweepResult :type "HitResult Structure (by ref)"))
  ;[1 1 1] Overlap Triggers
  (`KismetArrayLibrary.Array_Add` (`self.Components2`) OtherComp)
  (`KismetArrayLibrary.Array_AddUnique` (`self.CollisionIndexes`) 2))

(event `self.SphereCollision3.OnComponentBeginOverlap`
  (params (OverlappedComponent :type "PrimitiveComponent Object Reference") (OtherActor :type "Actor Object Reference") (OtherComp :type "PrimitiveComponent Object Reference") (OtherBodyIndex :type Integer) (bFromSweep :type Boolean) (SweepResult :type "HitResult Structure (by ref)"))
  ;[1 1 1] Overlap Triggers
  (`KismetArrayLibrary.Array_Add` (`self.Components3`) OtherComp)
  (`KismetArrayLibrary.Array_AddUnique` (`self.CollisionIndexes`) 3))

(event `self.SphereCollision4.OnComponentBeginOverlap`
  (params (OverlappedComponent :type "PrimitiveComponent Object Reference") (OtherActor :type "Actor Object Reference") (OtherComp :type "PrimitiveComponent Object Reference") (OtherBodyIndex :type Integer) (bFromSweep :type Boolean) (SweepResult :type "HitResult Structure (by ref)"))
  ;[1 1 1] Overlap Triggers
  (`KismetArrayLibrary.Array_Add` (`self.Components4`) OtherComp)
  (`KismetArrayLibrary.Array_AddUnique` (`self.CollisionIndexes`) 4))

(event `self.SphereCollision1.OnComponentEndOverlap`
  (params (OverlappedComponent :type "PrimitiveComponent Object Reference") (OtherActor :type "Actor Object Reference") (OtherComp :type "PrimitiveComponent Object Reference") (OtherBodyIndex :type Integer))
  (bind _components1 (`self.Components1`))
  ;[1 1 1] Overlap Triggers
  (`KismetArrayLibrary.Array_RemoveItem` _components1 OtherComp)
  (if (<= (`KismetArrayLibrary.Array_Length` _components1) 0)
    (`KismetArrayLibrary.Array_RemoveItem` (`self.CollisionIndexes`) 1)))

(event `self.SphereCollision2.OnComponentEndOverlap`
  (params (OverlappedComponent :type "PrimitiveComponent Object Reference") (OtherActor :type "Actor Object Reference") (OtherComp :type "PrimitiveComponent Object Reference") (OtherBodyIndex :type Integer))
  (bind _components2 (`self.Components2`))
  ;[1 1 1] Overlap Triggers
  (`KismetArrayLibrary.Array_RemoveItem` _components2 OtherComp)
  (if (<= (`KismetArrayLibrary.Array_Length` _components2) 0)
    (`KismetArrayLibrary.Array_RemoveItem` (`self.CollisionIndexes`) 2)))

(event `self.SphereCollision3.OnComponentEndOverlap`
  (params (OverlappedComponent :type "PrimitiveComponent Object Reference") (OtherActor :type "Actor Object Reference") (OtherComp :type "PrimitiveComponent Object Reference") (OtherBodyIndex :type Integer))
  (bind _components3 (`self.Components3`))
  ;[1 1 1] Overlap Triggers
  (`KismetArrayLibrary.Array_RemoveItem` _components3 OtherComp)
  (if (<= (`KismetArrayLibrary.Array_Length` _components3) 0)
    (`KismetArrayLibrary.Array_RemoveItem` (`self.CollisionIndexes`) 3)))

(event `self.SphereCollision4.OnComponentEndOverlap`
  (params (OverlappedComponent :type "PrimitiveComponent Object Reference") (OtherActor :type "Actor Object Reference") (OtherComp :type "PrimitiveComponent Object Reference") (OtherBodyIndex :type Integer))
  (bind _components4 (`self.Components4`))
  ;[1 1 1] Overlap Triggers
  (`KismetArrayLibrary.Array_RemoveItem` _components4 OtherComp)
  (if (<= (`KismetArrayLibrary.Array_Length` _components4) 0)
    (`KismetArrayLibrary.Array_RemoveItem` (`self.CollisionIndexes`) 4)
    (`PrimitiveComponent.SetMaterial` (`self.Tube90`) 0 "/Engine/EditorMeshes/ColorCalibrator/M_ClearCoat.M_ClearCoat")))

(event `AddForceToComponents`
  (bind _asstatic_mesh_component (cast `StaticMeshComponent` (`self.CurrentObject`)))
  (`PrimitiveComponent.AddForce` _asstatic_mesh_component (* (`SceneComponent.GetForwardVector` (`self.CurrentArrow`)) 8100.0) "None" false))

(event `GetComponentArray`
  (switch `int` (`self.Index`)
    (:`1`
      (set `self.CurrentComponentList` (`self.Components1`)))
    (:`2`
      (set `self.CurrentComponentList` (`self.Components2`)))
    (:`3`
      (set `self.CurrentComponentList` (`self.Components3`)))
    (:`4`
      (set `self.CurrentComponentList` (`self.Components4`)))))

(event `GetCurrentArrow`
  (bind _asarrow_component (cast `ArrowComponent` (`SceneComponent.GetChildComponent` (`SceneComponent.GetChildComponent` (`self.Tube90`) (- (`self.Index`) 1)) 0)))
  (set `self.CurrentArrow` _asarrow_component))

(fn `UserConstructionScript`)