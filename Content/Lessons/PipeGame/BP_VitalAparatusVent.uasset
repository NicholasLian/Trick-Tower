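; Vital apparatus vent actor for the pipe game lesson, with two semicircle halves that slide apart and close again when triggered.
; OpenVent records the trigger time and both halves' world positions, ignoring further calls while the motion runs.
; Tick derives a linear out-and-back offset from elapsed game time, moving the halves in opposite directions along world X for about two seconds, then restores their captured positions.
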(event `self.ReceiveTick`
  (params (DeltaSeconds :type "Float (single-precision)"))
  (bind _worldlocations (`self.WorldLocations`))
  (bind _percentage (`self.Percentage`))
  (bind _difference (`self.Difference`))
  (if (`self.CanOpen`)
    (bind _output_get (set `self.Difference` (- (`KismetSystemLibrary.GetGameTimeInSeconds`) (`self.TriggerTime`))))
    (if (<= _output_get 2.0)
      (if (<= _output_get 1.0)
        (set `self.Percentage` _difference)
        (else
          (set `self.Percentage` (- 2.0 _difference))))
      (else
        (set `self.CanOpen` false)
        (set `self.Percentage` 0.0)))
    (`SceneComponent.K2_SetWorldLocation` (`self.SemicircleL`) (+ (`KismetArrayLibrary.Array_Get` _worldlocations) (`KismetMathLibrary.MakeVector` (* _percentage -100.0))) false false)
    (`SceneComponent.K2_SetWorldLocation` (`self.SemicircleR`) (+ (`KismetArrayLibrary.Array_Get` _worldlocations 1) (`KismetMathLibrary.MakeVector` (* _percentage 100.0))) false false)))

(event `OpenVent`
  (if (not (`self.CanOpen`))
    (set `self.CanOpen` true)
    (set `self.TriggerTime` (`KismetSystemLibrary.GetGameTimeInSeconds`))
    (set `self.WorldLocations` (`|MakeArray` (`SceneComponent.K2_GetComponentLocation` (`self.SemicircleL`)) (`SceneComponent.K2_GetComponentLocation` (`self.SemicircleR`))))))

(fn `UserConstructionScript`)