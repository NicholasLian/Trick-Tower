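; BP_MemoryCube holds the selection state for a pipe puzzle, tracking the current cell in a 5x5 grid.
; ToggleX and ToggleY step within the grid, then update the current actor and camera from per-row arrays indexed by X and teleport the BP_TubeBracket indicator to the cell.
; RotateCurrentActorEvent sends a vent-rotation interface message to the selected actor, and RetrieveMemory returns the current actor and camera.
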(event `self.ReceiveBeginPlay`
  (set `self.X` 0)
  (set `self.Y` 0)
  (set `self.CurrentActor` (`KismetArrayLibrary.Array_Get` (`self.Actors0`)))
  (set `self.CurrentCamera` (`KismetArrayLibrary.Array_Get` (`self.Cameras0`))))

(event `ToggleX`
  (params (IsIncrease :type Boolean))
  (bind _x (`self.X`))
  (if IsIncrease
    (if (< _x 4)
      (bind _result (`/Engine/EditorBlueprintResources/StandardMacros.IncrementInt` _x)
        (:`  `
          (set `self.X` _result)
          (`self.SetCurrentActorEvent` :!label _label)
          (`self.SetTubeIndicatorLocation`)
          (`self.SetCurrentCameraEvent`))))
    (elif (> _x 0)
      (bind _result_2 (`/Engine/EditorBlueprintResources/StandardMacros.DecrementInt` _x)
        (:`  `
          (set `self.X` _result_2)
          (goto _label))))))

(event `ToggleY`
  (params (IsIncrease :type Boolean))
  (bind _y (`self.Y`))
  (if IsIncrease
    (if (< _y 4)
      (bind _result (`/Engine/EditorBlueprintResources/StandardMacros.IncrementInt` _y)
        (:`  `
          (set `self.Y` _result)
          (goto _label))))
    (elif (> _y 0)
      (bind _result_2 (`/Engine/EditorBlueprintResources/StandardMacros.DecrementInt` _y)
        (:`  `
          (set `self.Y` _result_2)
          (goto _label))))))

(event `SetCurrentActorEvent`
  (bind _x (`self.X`))
  (switch `int` (`self.Y`)
    (:`0`
      (set `self.CurrentActor` (`KismetArrayLibrary.Array_Get` (`self.Actors0`) _x)))
    (:`1`
      (set `self.CurrentActor` (`KismetArrayLibrary.Array_Get` (`self.Actors1`) _x)))
    (:`2`
      (set `self.CurrentActor` (`KismetArrayLibrary.Array_Get` (`self.Actors2`) _x)))
    (:`3`
      (set `self.CurrentActor` (`KismetArrayLibrary.Array_Get` (`self.Actors3`) _x)))
    (:`4`
      (set `self.CurrentActor` (`KismetArrayLibrary.Array_Get` (`self.Actors4`) _x)))))

(event `SetTubeIndicatorLocation`
  (bind _returnvalue (`KismetMathLibrary.SelectFloat` 325.0 0.0 true))
  (bind _asbp_tube_bracket (cast `/Game/Lessons/PipeGame/BP_TubeBracket` (`self.TubeIndicator`)))
  (`self.K2_SetActorLocation` _asbp_tube_bracket (`KismetMathLibrary.MakeVector` (- 650.0 (* (`self.X`) _returnvalue)) (* (`self.Y`) _returnvalue) 265.0) false true))

(event `RotateCurrentActorEvent`
  (message `/Game/Lessons/PipeGame/BPI_RotateVentInterface.RotateVentInterface` (`self.CurrentActor`)))

(event `SetCurrentCameraEvent`
  (bind _x (`self.X`))
  (switch `int` (`self.Y`)
    (:`0`
      (set `self.CurrentCamera` (`KismetArrayLibrary.Array_Get` (`self.Cameras0`) _x)))
    (:`1`
      (set `self.CurrentCamera` (`KismetArrayLibrary.Array_Get` (`self.Cameras1`) _x)))
    (:`2`
      (set `self.CurrentCamera` (`KismetArrayLibrary.Array_Get` (`self.Cameras2`) _x)))
    (:`3`
      (set `self.CurrentCamera` (`KismetArrayLibrary.Array_Get` (`self.Cameras3`) _x)))
    (:`4`
      (set `self.CurrentCamera` (`KismetArrayLibrary.Array_Get` (`self.Cameras4`) _x)))))

(fn `RetrieveMemory`
  (returns (CurrentActor :type "Actor Object Reference") (CurrentCamera :type "/Game/Lessons/PipeGame/BP_StationaryCamera Object Reference"))
  (return (`self.CurrentActor`) (`self.CurrentCamera`)))

(fn `UserConstructionScript`)