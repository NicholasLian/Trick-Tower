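; Torus goalpost for the pipe game that marks a goal as achieved and brings in the next level.
; Any overlap with its sphere collision turns the torus and goal indicator blue, stores the overlapping component and timestamps the trigger.
; Tick then drives a time-based two-stage animation, yawing the rotating wall a quarter turn, then sliding the next level along negative Y.
; ActNow starts the same sequence without the material changes.
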(event `self.ReceiveBeginPlay`
  (set `self.NextLevelLocation` (`SceneComponent.K2_GetComponentLocation` (`/Game/Lessons/ProjectLevel/BP_NextLevel.DefaultSceneRoot` (`self.NextLevel`))))
  (set `self.RotatingWallRotation` (`SceneComponent.K2_GetComponentRotation` (`/Game/Lessons/PipeGame/BP_RotatingWall.DefaultSceneRoot` (`self.RotatingWall`)))))

(event `self.ReceiveTick`
  (params (DeltaSeconds :type "Float (single-precision)"))
  (if (`self.GoalAchieved`)
    (`self.RotateWall`)))

(event `self.SphereCollision.OnComponentBeginOverlap`
  (params (OverlappedComponent :type "PrimitiveComponent Object Reference") (OtherActor :type "Actor Object Reference") (OtherComp :type "PrimitiveComponent Object Reference") (OtherBodyIndex :type Integer) (bFromSweep :type Boolean) (SweepResult :type "HitResult Structure (by ref)"))
  (`KismetArrayLibrary.Array_Add` (`self.Components`) OtherComp)
  (`PrimitiveComponent.SetMaterial` (`self.Torus`) 0 "/Game/Materials/Architecture/Sci-Fi/Unique/MI_Wall_Blue_Solid.MI_Wall_Blue_Solid")
  (`PrimitiveComponent.SetMaterial` (`/Game/Lessons/PipeGame/BP_GoalIndicator.StaticMesh` (`self.GoalIndicator`)) 0 "/Engine/EngineDebugMaterials/VertexColorViewMode_BlueOnly.VertexColorViewMode_BlueOnly")
  (set `self.GoalAchieved` true)
  (set `self.TriggerTime` (`KismetSystemLibrary.GetGameTimeInSeconds`)))

(event `RotateWall`
  (bind _returnvalue (- (`KismetSystemLibrary.GetGameTimeInSeconds`) (`self.TriggerTime`)))
  (if (<= _returnvalue 1.0)
    (`SceneComponent.K2_SetWorldRotation` (`/Game/Lessons/PipeGame/BP_RotatingWall.DefaultSceneRoot` (`self.RotatingWall`)) (`KismetMathLibrary.ComposeRotators` (`self.RotatingWallRotation`) (`KismetMathLibrary.MakeRotator` 0.0 0.0 (* _returnvalue 90.0))) false false)
    (elif (<= _returnvalue 2.0)
      (`SceneComponent.K2_SetWorldLocation` (`/Game/Lessons/ProjectLevel/BP_NextLevel.DefaultSceneRoot` (`self.NextLevel`)) (+ (`self.NextLevelLocation`) (`KismetMathLibrary.MakeVector` 0.0 (* (- _returnvalue 1.0) -300.0))) false false))))

(event `ActNow`
  (set `self.GoalAchieved` true)
  (set `self.TriggerTime` (`KismetSystemLibrary.GetGameTimeInSeconds`)))

(fn `UserConstructionScript`)