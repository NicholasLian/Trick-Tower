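; Pipe-game piece with two 90-degree tubes (SE and NW) that pushes static mesh components through them.
; Four sphere triggers per tube track overlapping components and active indices, and each tube's first trigger switches it to clear glass.
; Tick applies a constant force along each active sphere's child arrow to its components.
; B2 registers as index 5 instead of 6, and A2's end overlap removes 1 instead of 2.
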(event `self.ReceiveBeginPlay`
  (set `self.Index` 0))

(event `self.ReceiveTick`
  (params (DeltaSeconds :type "Float (single-precision)"))
  (for _array_element (`self.CollisionIndexes`)
    (set `self.Index` _array_element) ; Represents Current Sphere Collision
    (`self.GetComponentArray`)
    (`self.GetCurrentArrow`)
    (for _array_element_2 (`self.CurrentComponentList`)
      (set `self.CurrentObject` _array_element_2)
      (`self.AddForceToComponents`))))

(event `self.SphereCollisionA1.OnComponentBeginOverlap`
  (params (OverlappedComponent :type "PrimitiveComponent Object Reference") (OtherActor :type "Actor Object Reference") (OtherComp :type "PrimitiveComponent Object Reference") (OtherBodyIndex :type Integer) (bFromSweep :type Boolean) (SweepResult :type "HitResult Structure (by ref)"))
  ;[1 1 1] Overlap Triggers
  (`KismetArrayLibrary.Array_Add` (`self.ComponentsA1`) OtherComp)
  (`KismetArrayLibrary.Array_AddUnique` (`self.CollisionIndexes`) 1)
  (`PrimitiveComponent.SetMaterial` (`self.Tube90SE`) 0 "/Game/Materials/Architecture/Glass/MI_Glass_Clear.MI_Glass_Clear"))

(event `self.SphereCollisionA2.OnComponentBeginOverlap`
  (params (OverlappedComponent :type "PrimitiveComponent Object Reference") (OtherActor :type "Actor Object Reference") (OtherComp :type "PrimitiveComponent Object Reference") (OtherBodyIndex :type Integer) (bFromSweep :type Boolean) (SweepResult :type "HitResult Structure (by ref)"))
  ;[1 1 1] Overlap Triggers
  (`KismetArrayLibrary.Array_Add` (`self.ComponentsA2`) OtherComp)
  (`KismetArrayLibrary.Array_AddUnique` (`self.CollisionIndexes`) 2))

(event `self.SphereCollisionA3.OnComponentBeginOverlap`
  (params (OverlappedComponent :type "PrimitiveComponent Object Reference") (OtherActor :type "Actor Object Reference") (OtherComp :type "PrimitiveComponent Object Reference") (OtherBodyIndex :type Integer) (bFromSweep :type Boolean) (SweepResult :type "HitResult Structure (by ref)"))
  ;[1 1 1] Overlap Triggers
  (`KismetArrayLibrary.Array_Add` (`self.ComponentsA3`) null)
  (`KismetArrayLibrary.Array_AddUnique` (`self.CollisionIndexes`) 3))

(event `self.SphereCollisionA4.OnComponentBeginOverlap`
  (params (OverlappedComponent :type "PrimitiveComponent Object Reference") (OtherActor :type "Actor Object Reference") (OtherComp :type "PrimitiveComponent Object Reference") (OtherBodyIndex :type Integer) (bFromSweep :type Boolean) (SweepResult :type "HitResult Structure (by ref)"))
  ;[1 1 1] Overlap Triggers
  (`KismetArrayLibrary.Array_Add` (`self.ComponentsA4`) OtherComp)
  (`KismetArrayLibrary.Array_AddUnique` (`self.CollisionIndexes`) 4))

(event `self.SphereCollisionA1.OnComponentEndOverlap`
  (params (OverlappedComponent :type "PrimitiveComponent Object Reference") (OtherActor :type "Actor Object Reference") (OtherComp :type "PrimitiveComponent Object Reference") (OtherBodyIndex :type Integer))
  (bind _componentsa1 (`self.ComponentsA1`))
  ;[1 1 1] Overlap Triggers
  (`KismetArrayLibrary.Array_RemoveItem` _componentsa1 OtherComp)
  (if (<= (`KismetArrayLibrary.Array_Length` _componentsa1) 0)
    (`KismetArrayLibrary.Array_RemoveItem` (`self.CollisionIndexes`) 1)))

(event `self.SphereCollisionA2.OnComponentEndOverlap`
  (params (OverlappedComponent :type "PrimitiveComponent Object Reference") (OtherActor :type "Actor Object Reference") (OtherComp :type "PrimitiveComponent Object Reference") (OtherBodyIndex :type Integer))
  (bind _componentsa2 (`self.ComponentsA2`))
  ;[1 1 1] Overlap Triggers
  (`KismetArrayLibrary.Array_RemoveItem` _componentsa2 OtherComp)
  (if (<= (`KismetArrayLibrary.Array_Length` _componentsa2) 0)
    (`KismetArrayLibrary.Array_RemoveItem` (`self.CollisionIndexes`) 1)))

(event `self.SphereCollisionA3.OnComponentEndOverlap`
  (params (OverlappedComponent :type "PrimitiveComponent Object Reference") (OtherActor :type "Actor Object Reference") (OtherComp :type "PrimitiveComponent Object Reference") (OtherBodyIndex :type Integer))
  (bind _componentsa3 (`self.ComponentsA3`))
  ;[1 1 1] Overlap Triggers
  (`KismetArrayLibrary.Array_RemoveItem` _componentsa3 null)
  (if (<= (`KismetArrayLibrary.Array_Length` _componentsa3) 0)
    (`KismetArrayLibrary.Array_RemoveItem` (`self.CollisionIndexes`) 3)))

(event `self.SphereCollisionA4.OnComponentEndOverlap`
  (params (OverlappedComponent :type "PrimitiveComponent Object Reference") (OtherActor :type "Actor Object Reference") (OtherComp :type "PrimitiveComponent Object Reference") (OtherBodyIndex :type Integer))
  (bind _componentsa4 (`self.ComponentsA4`))
  ;[1 1 1] Overlap Triggers
  (`KismetArrayLibrary.Array_RemoveItem` _componentsa4 OtherComp)
  (if (<= (`KismetArrayLibrary.Array_Length` _componentsa4) 0)
    (`KismetArrayLibrary.Array_RemoveItem` (`self.CollisionIndexes`) 4)))

(event `self.SphereCollisionB1.OnComponentBeginOverlap`
  (params (OverlappedComponent :type "PrimitiveComponent Object Reference") (OtherActor :type "Actor Object Reference") (OtherComp :type "PrimitiveComponent Object Reference") (OtherBodyIndex :type Integer) (bFromSweep :type Boolean) (SweepResult :type "HitResult Structure (by ref)"))
  ;[1 1 1] Overlap Triggers
  (`KismetArrayLibrary.Array_Add` (`self.ComponentsB1`) OtherComp)
  (`KismetArrayLibrary.Array_AddUnique` (`self.CollisionIndexes`) 5)
  (`PrimitiveComponent.SetMaterial` (`self.Tube90NW`) 0 "/Game/Materials/Architecture/Glass/MI_Glass_Clear.MI_Glass_Clear"))

(event `self.SphereCollisionB2.OnComponentBeginOverlap`
  (params (OverlappedComponent :type "PrimitiveComponent Object Reference") (OtherActor :type "Actor Object Reference") (OtherComp :type "PrimitiveComponent Object Reference") (OtherBodyIndex :type Integer) (bFromSweep :type Boolean) (SweepResult :type "HitResult Structure (by ref)"))
  ;[1 1 1] Overlap Triggers
  (`KismetArrayLibrary.Array_Add` (`self.ComponentsB2`) OtherComp)
  (`KismetArrayLibrary.Array_AddUnique` (`self.CollisionIndexes`) 5))

(event `self.SphereCollisionB3.OnComponentBeginOverlap`
  (params (OverlappedComponent :type "PrimitiveComponent Object Reference") (OtherActor :type "Actor Object Reference") (OtherComp :type "PrimitiveComponent Object Reference") (OtherBodyIndex :type Integer) (bFromSweep :type Boolean) (SweepResult :type "HitResult Structure (by ref)"))
  ;[1 1 1] Overlap Triggers
  (`KismetArrayLibrary.Array_Add` (`self.ComponentsB3`) OtherComp)
  (`KismetArrayLibrary.Array_AddUnique` (`self.CollisionIndexes`) 7))

(event `self.SphereCollisionB4.OnComponentBeginOverlap`
  (params (OverlappedComponent :type "PrimitiveComponent Object Reference") (OtherActor :type "Actor Object Reference") (OtherComp :type "PrimitiveComponent Object Reference") (OtherBodyIndex :type Integer) (bFromSweep :type Boolean) (SweepResult :type "HitResult Structure (by ref)"))
  ;[1 1 1] Overlap Triggers
  (`KismetArrayLibrary.Array_Add` (`self.ComponentsB4`) OtherComp)
  (`KismetArrayLibrary.Array_AddUnique` (`self.CollisionIndexes`) 8))

(event `self.SphereCollisionB1.OnComponentEndOverlap`
  (params (OverlappedComponent :type "PrimitiveComponent Object Reference") (OtherActor :type "Actor Object Reference") (OtherComp :type "PrimitiveComponent Object Reference") (OtherBodyIndex :type Integer))
  (bind _componentsb1 (`self.ComponentsB1`))
  ;[1 1 1] Overlap Triggers
  (`KismetArrayLibrary.Array_RemoveItem` _componentsb1 OtherComp)
  (if (<= (`KismetArrayLibrary.Array_Length` _componentsb1) 0)
    (`KismetArrayLibrary.Array_RemoveItem` (`self.CollisionIndexes`) 5)))

(event `self.SphereCollisionB2.OnComponentEndOverlap`
  (params (OverlappedComponent :type "PrimitiveComponent Object Reference") (OtherActor :type "Actor Object Reference") (OtherComp :type "PrimitiveComponent Object Reference") (OtherBodyIndex :type Integer))
  (bind _componentsb2 (`self.ComponentsB2`))
  ;[1 1 1] Overlap Triggers
  (`KismetArrayLibrary.Array_RemoveItem` _componentsb2 OtherComp)
  (if (<= (`KismetArrayLibrary.Array_Length` _componentsb2) 0)
    (`KismetArrayLibrary.Array_RemoveItem` (`self.CollisionIndexes`) 5)))

(event `self.SphereCollisionB3.OnComponentEndOverlap`
  (params (OverlappedComponent :type "PrimitiveComponent Object Reference") (OtherActor :type "Actor Object Reference") (OtherComp :type "PrimitiveComponent Object Reference") (OtherBodyIndex :type Integer))
  (bind _componentsb3 (`self.ComponentsB3`))
  ;[1 1 1] Overlap Triggers
  (`KismetArrayLibrary.Array_RemoveItem` _componentsb3 OtherComp)
  (if (<= (`KismetArrayLibrary.Array_Length` _componentsb3) 0)
    (`KismetArrayLibrary.Array_RemoveItem` (`self.CollisionIndexes`) 7)))

(event `self.SphereCollisionB4.OnComponentEndOverlap`
  (params (OverlappedComponent :type "PrimitiveComponent Object Reference") (OtherActor :type "Actor Object Reference") (OtherComp :type "PrimitiveComponent Object Reference") (OtherBodyIndex :type Integer))
  (bind _componentsb4 (`self.ComponentsB4`))
  ;[1 1 1] Overlap Triggers
  (`KismetArrayLibrary.Array_RemoveItem` _componentsb4 OtherComp)
  (if (<= (`KismetArrayLibrary.Array_Length` _componentsb4) 0)
    (`KismetArrayLibrary.Array_RemoveItem` (`self.CollisionIndexes`) 8)))

(event `AddForceToComponents`
  (bind _asstatic_mesh_component (cast `StaticMeshComponent` (`self.CurrentObject`)))
  (`PrimitiveComponent.AddForce` _asstatic_mesh_component (* (`SceneComponent.GetForwardVector` (`self.CurrentArrow`)) 640000.0) "None" false))

(event `GetComponentArray`
  (switch `int` (`self.Index`)
    (:`1`
      (set `self.CurrentComponentList` (`self.ComponentsA1`)))
    (:`2`
      (set `self.CurrentComponentList` (`self.ComponentsA2`)))
    (:`3`
      (set `self.CurrentComponentList` (`self.ComponentsA3`)))
    (:`4`
      (set `self.CurrentComponentList` (`self.ComponentsA4`)))
    (:`5`
      (set `self.CurrentComponentList` (`self.ComponentsB1`)))
    (:`6`
      (set `self.CurrentComponentList` (`self.ComponentsB2`)))
    (:`7`
      (set `self.CurrentComponentList` (`self.ComponentsB3`)))
    (:`8`
      (set `self.CurrentComponentList` (`self.ComponentsB4`)))))

(event `GetCurrentArrow`
  (bind _index (`self.Index`))
  (if (<= _index 4)
    (bind _asarrow_component (cast `ArrowComponent` (`SceneComponent.GetChildComponent` (`SceneComponent.GetChildComponent` (`self.Tube90SE`) (- _index 1)) 0)))
    (set `self.CurrentArrow` _asarrow_component)
    (else
      (bind _asarrow_component_2 (cast `ArrowComponent` (`SceneComponent.GetChildComponent` (`SceneComponent.GetChildComponent` (`self.Tube90NW`) (- _index 5)) 0)))
      (set `self.CurrentArrow` _asarrow_component_2))))

(fn `UserConstructionScript`)