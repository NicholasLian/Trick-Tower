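; BP_NormalCube is a cube that reveals a bomb number and changes material once something overlaps its box, suggesting a safe tile in a Minesweeper-style game.
; BeginPlay writes the BombNum value into the text component.
; The box overlap latches an Overlapped flag, and Tick polls it to show the text and swap the material once, guarded by a Changed flag.
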(event `self.ReceiveBeginPlay`
  (`TextRenderComponent.K2_SetText` (`self.BombNum`) (`KismetTextLibrary.Conv_IntToText` (`self.bomb_num`))))

(event `self.ReceiveTick`
  (params (DeltaSeconds :type "Float (single-precision)"))
  (if (`self.overlapped`)
    (if (not (`self.changed`))
      (`SceneComponent.SetVisibility` (`self.BombNum`) true false)
      (`PrimitiveComponent.SetMaterial` (`self.Cube`) 0 "/Game/Lessons/Materials/Architecture/Metal/Bare/MI_Metal_Powder_001_a.MI_Metal_Powder_001_a")
      (set `self.changed` true))))

(event `self.Box.OnComponentBeginOverlap`
  (params (OverlappedComponent :type "PrimitiveComponent Object Reference") (OtherActor :type "Actor Object Reference") (OtherComp :type "PrimitiveComponent Object Reference") (OtherBodyIndex :type Integer) (bFromSweep :type Boolean) (SweepResult :type "HitResult Structure (by ref)"))
  (if (not (`self.overlapped`))
    (set `self.overlapped` true)))

(fn `UserConstructionScript`)