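; BP_BombCube is a cube actor that explodes and removes itself after something overlaps its box.
; The box overlap swaps the cube's material and sets an Overlapped flag.
; Tick polls that flag, spawning a neon explosion emitter and sound at the actor's location, then destroys the actor after a short delay.
; The flag is never cleared, so both effects respawn every frame until destruction.
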(event `self.ReceiveTick`
  (params (DeltaSeconds :type "Float (single-precision)"))
  (bind _returnvalue (`self.K2_GetActorLocation`))
  (if (`self.overlapped`)
    (`GameplayStatics.SpawnEmitterAtLocation` "/Game/Effects/Particles/Explosion/P_NeonExplosion.P_NeonExplosion" _returnvalue)
    (`GameplayStatics.SpawnSoundAtLocation` "/Game/Audio/SoundWaves/Effect/SW_Explosion_1.SW_Explosion_1" _returnvalue)
    (`KismetSystemLibrary.Delay` 0.5)
    (`self.K2_DestroyActor`)))

(event `self.Box.OnComponentBeginOverlap`
  (params (OverlappedComponent :type "PrimitiveComponent Object Reference") (OtherActor :type "Actor Object Reference") (OtherComp :type "PrimitiveComponent Object Reference") (OtherBodyIndex :type Integer) (bFromSweep :type Boolean) (SweepResult :type "HitResult Structure (by ref)"))
  (`PrimitiveComponent.SetMaterial` (`self.Cube`) 0 "/Game/Lessons/Materials/Architecture/BuildingBlocks/MI_Prototyper_ObjectSpace.MI_Prototyper_ObjectSpace")
  (set `self.overlapped` true))

(fn `UserConstructionScript`)