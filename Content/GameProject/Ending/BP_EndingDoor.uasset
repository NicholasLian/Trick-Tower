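; BP_EndingDoor is a door actor for the game's ending that rises upward once when activated.
; BeginPlay caches the starting location, and OnActivate plays a chime and runs the Movement timeline, which offsets the actor vertically from that location.
; An IsActivated flag, set as the timeline updates, blocks repeat activation.
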(event `OnActivate`
  (if (not (`self.isActivated`))
    (`GameplayStatics.PlaySoundAtLocation` "/Game/Audio/SoundWaves/Effect/SW_Chime_1.SW_Chime_1" (`self.K2_GetActorLocation`))
    (bind (_direction _position) (`Timeline|Movement`)
      (:`Update`
        (`self.K2_SetActorLocation` (+ (`self.InitialLocation`) (* (0.0 0.0 300.0) _position)))
        (set `self.isActivated` true)))))

(event `self.ReceiveBeginPlay`
  (set `self.InitialLocation` (`self.K2_GetActorLocation`)))

(fn `UserConstructionScript`)