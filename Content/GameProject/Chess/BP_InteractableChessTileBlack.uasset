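; Black chess tile trigger that activates a linked door when stood on for three seconds.
; Box overlap starts a timer accumulated in Tick and leaving resets it, with no check on which actor overlaps.
; At the threshold it calls OnActivate on ActivatingDoor and destroys the Box, making the trigger one-shot.
; A chime and "Correct Answer" print are present but disconnected, so they never run.
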(event `self.ReceiveTick`
  (params (DeltaSeconds :type "Float (single-precision)"))
  (if (`self.playerIsStepping`)
    (bind _output_get (set `self.timePlayerIsStepping` (+ DeltaSeconds (`self.timePlayerIsStepping`))))
    (if (>= _output_get 3.0)
      (`/Game/GameProject/Chess/BP_PuzzleDoor.OnActivate` (`self.activatingDoor`))
      (`ActorComponent.K2_DestroyComponent` (`self.Box`)))))

(event `self.Box.OnComponentBeginOverlap`
  (params (OverlappedComponent :type "PrimitiveComponent Object Reference") (OtherActor :type "Actor Object Reference") (OtherComp :type "PrimitiveComponent Object Reference") (OtherBodyIndex :type Integer) (bFromSweep :type Boolean) (SweepResult :type "HitResult Structure (by ref)"))
  (set `self.playerIsStepping` true))

(event `self.Box.OnComponentEndOverlap`
  (params (OverlappedComponent :type "PrimitiveComponent Object Reference") (OtherActor :type "Actor Object Reference") (OtherComp :type "PrimitiveComponent Object Reference") (OtherBodyIndex :type Integer))
  (set `self.playerIsStepping` false)
  (set `self.timePlayerIsStepping` 0.0))

(fn `UserConstructionScript`)